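; Base enemy character that walks when able to act, damages the hero on contact, and reacts to being hit.
; Hurtbox overlap applies damage only when it touches the hero's own Hurtbox.
; The extended hit handler adds hit stop and a retriggerable timed stun, then checks the health component for defeat.
; Defeat disables Hurtbox collision, waits a despawn delay, then spawns a skull explosion effect and destroys the actor.
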(event `WalkTowards`
  (params (WorldDirection :type "Vector Structure"))
  (if (`self.Can Act`)
    (`self.AddMovementInput` WorldDirection)))

(event `self.Hurtbox.OnComponentBeginOverlap`
  (params (OverlappedComponent :type "PrimitiveComponent Object Reference") (OtherActor :type "Actor Object Reference") (OtherComp :type "PrimitiveComponent Object Reference") (OtherBodyIndex :type Integer) (bFromSweep :type Boolean) (SweepResult :type "HitResult Structure (by ref)"))
  (bind _asbp_hero (cast `/Game/Dynamic/Blueprints/Characters/Hero/BP_Hero` OtherActor))
  (if (== (`/Game/Dynamic/Blueprints/Characters/BP_DungeonChar_BASE.Hurtbox` _asbp_hero) OtherComp)
    (`GameplayStatics.ApplyDamage` _asbp_hero 1.0 null self)))

(event `SetStun`
  (set `self.isStunned` true)
  (`KismetSystemLibrary.RetriggerableDelay` (`self.StunDuration`))
  (set `self.isStunned` false))

(event `HandleDefeat`
  (`PrimitiveComponent.SetCollisionEnabled` (`self.Hurtbox`) "NoCollision")
  (`KismetSystemLibrary.Delay` (`self.DespawnDelay`))
  (`|SpawnActorFromClass` "/Game/Dynamic/Blueprints/VFX/BP_VFX_SkullExplosion.BP_VFX_SkullExplosion_C" (`KismetMathLibrary.MakeTransform` (`self.K2_GetActorLocation`)) "AlwaysSpawn" "MultiplyWithRoot" null null)
  (`self.K2_DestroyActor`))

(fn `HandleHitExtended`
  (`parent.HandleHitExtended`)
  (`self.HitStop`)
  (`self.SetStun`)
  (if (`/Game/Dynamic/Blueprints/Components/BPC_Health.IsDefeated` (`self.BPC_Health`))
    (`self.HandleDefeat`)))

(fn `UserConstructionScript`
  (`parent.UserConstructionScript`))