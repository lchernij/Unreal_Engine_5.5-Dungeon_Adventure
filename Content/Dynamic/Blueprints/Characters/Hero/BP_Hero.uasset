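; BP_Hero is the player character, with Enhanced Input movement, sword and bow attacks played as sprite animation overrides.
; CheckHit damages enemies overlapping the hitbox, and FireArrow spawns arrow projectiles.
; Getting hit updates the HUD hearts, disables the hurtbox and stuns until the hit animation ends, then jumps to defeat or flickers the sprite until health-component invincibility expires.
; GetHealed raises health and refreshes the HUD.
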(event `self.ReceiveBeginPlay`
  (`|ExecutionSequence`
    (:`then_0`
      (bind _asplayer_controller (cast `PlayerController` (`self.GetController`)))
      (`EnhancedInputSubsystemInterface.AddMappingContext` (pcsubsystem `EnhancedInputLocalPlayerSubsystem` _asplayer_controller) "/Game/Dynamic/Input/IMC_Dungeon.IMC_Dungeon" 0 (struct)))
    (:`then_1`
      (add `/Game/Dynamic/Blueprints/Components/BPC_Health.InvincibilityExpired` (`self.BPC_Health`) (delegate `OnInvincibilityExpired`)))
    (:`then_2`
      (bind _returnvalue (`|CreateWidget` "/Game/Dynamic/Widgets/WBP_MainHUD.WBP_MainHUD_C"))
      (bind _output_get (set `self.MainHUD` _returnvalue))
      (`UserWidget.AddToViewport` _output_get 0)
      (`/Game/Dynamic/Widgets/WBP_HealthBox.InitialHeartPieces` (`/Game/Dynamic/Widgets/WBP_MainHUD.WBP_HealthBox` (`self.MainHUD`)) (`/Game/Dynamic/Blueprints/Components/BPC_Health.MaxHealth` (`self.BPC_Health`))))
    (:`then_3`
      (`SceneComponent.K2_SetWorldLocation` (`self.SpringArm`) (`self.K2_GetActorLocation`) false false))))

(event `OnInvincibilityExpired`
  (`KismetSystemLibrary.K2_ClearAndInvalidateTimerHandle` (`self.FlickerHandler`))
  (`SceneComponent.SetVisibility` (`self.Sprite`) true false)
  (`PrimitiveComponent.SetCollisionEnabled` (`self.Hurtbox`) "QueryOnly"))

(event `EnhancedInput|/Game/Dynamic/Input/Actions/IA_Move`
  (params (ActionValue :type "Vector2D Structure") (ElapsedSeconds :type "Float (double-precision)") (TriggeredSeconds :type "Float (double-precision)") (InputAction :type "InputAction Object Reference" :default "/Game/Dynamic/Input/Actions/IA_Move.IA_Move"))
  (bind (_x _y) (`KismetMathLibrary.BreakVector2D` ActionValue))
  (:`Triggered`
    (if (`self.Can Act`)
      (set `self.Directionality` ActionValue)
      (`self.AddMovementInput` (1.0 0.0 0.0) _x)
      (`self.AddMovementInput` (0.0 1.0 0.0) _y))))

(event `EnhancedInput|/Game/Dynamic/Input/Actions/IA_Sword`
  (params (ActionValue :type Boolean) (ElapsedSeconds :type "Float (double-precision)") (TriggeredSeconds :type "Float (double-precision)") (InputAction :type "InputAction Object Reference" :default "/Game/Dynamic/Input/Actions/IA_Sword.IA_Sword"))
  (:`Started`
    (if (`self.Can Act`)
      (`PaperZDPlaySlotOverrideAction.PlayAnimationOverrideWithCallbacks` (`PaperZDAnimationComponent.AnimInstance` (`self.AnimationComponent`)) "/Game/Dynamic/Blueprints/Characters/Hero/AnimSequences/Attack.Attack" "DefaultSlot" (`self.Sword Play Rate`)
        (:`then`
          (set `self.isAttacking` true))
        (:`OnCompleted`
          (set `self.isAttacking` false :!label _label))
        (:`OnCancelled`
          (goto _label))))))

(event `EnhancedInput|/Game/Dynamic/Input/Actions/IA_Bow`
  (params (ActionValue :type Boolean) (ElapsedSeconds :type "Float (double-precision)") (TriggeredSeconds :type "Float (double-precision)") (InputAction :type "InputAction Object Reference" :default "/Game/Dynamic/Input/Actions/IA_Bow.IA_Bow"))
  (:`Triggered`
    (if (and (`self.Can Act`) (`self.CanUseBow`))
      (`PaperZDPlaySlotOverrideAction.PlayAnimationOverrideWithCallbacks` (`PaperZDAnimationComponent.AnimInstance` (`self.AnimationComponent`)) "/Game/Dynamic/Blueprints/Characters/Hero/AnimSequences/Bow.Bow"
        (:`then`
          (set `self.isAttacking` true))
        (:`OnCompleted`
          (set `self.isAttacking` false :!label _label_2))
        (:`OnCancelled`
          (goto _label_2))))))

(event `self.HandleHitExtended`
  (`parent.HandleHitExtended`)
  (`/Game/Dynamic/Widgets/WBP_HealthBox.UpdateCurrentHealth` (`/Game/Dynamic/Widgets/WBP_MainHUD.WBP_HealthBox` (`self.MainHUD`)) (`/Game/Dynamic/Blueprints/Components/BPC_Health.CurrentHealth` (`self.BPC_Health`)))
  (`/Game/Dynamic/Blueprints/Components/BPC_Health.SetInvincibility` (`self.BPC_Health`))
  (`PrimitiveComponent.SetCollisionEnabled` (`self.Hurtbox`) "NoCollision")
  (`PaperZDPlaySlotOverrideAction.PlayAnimationOverrideWithCallbacks` (`PaperZDAnimationComponent.AnimInstance` (`self.AnimationComponent`)) (`self.GetHitAnimation`)
    (:`then`
      (set `self.isStunned` true))
    (:`OnCompleted`
      (set `self.isStunned` false :!label _label_3)
      (`self.HitStop`)
      (if (`/Game/Dynamic/Blueprints/Components/BPC_Health.IsDefeated` (`self.BPC_Health`))
        (`PaperZDAnimInstance.JumpToNode` (`PaperZDAnimationComponent.AnimInstance` (`self.AnimationComponent`)) "DefeatJump" "None")
        (else
          (bind _returnvalue (`KismetSystemLibrary.K2_SetTimerDelegate` (`|CreateDelegate` :!event `SetSpriteVisibility`) (`self.SpriteFlickerInterval`) true))
          (set `self.FlickerHandler` _returnvalue))))
    (:`OnCancelled`
      (goto _label_3))))

(fn `CheckHit`
  (bind (_arrayindex _arrayelement) (`/Engine/EditorBlueprintResources/StandardMacros.ReverseForEachLoop` (`PrimitiveComponent.GetOverlappingActors` (`self.Hitbox`) "/Game/Dynamic/Blueprints/Characters/BP_Enemy_BASE.BP_Enemy_BASE_C"))
    (:`LoopBody`
      (`GameplayStatics.ApplyDamage` _arrayelement (`self.SwordDamage`) null self))))

(fn `FireArrow`
  (bind (_returnvalue_location _returnvalue_rotation) (`KismetMathLibrary.BreakTransform` (`SceneComponent.K2_GetComponentToWorld` (`self.ArrowPos`))))
  (`|SpawnActorFromClass` "/Game/Dynamic/Blueprints/Projectiles/BP_Projectiles_Arrow.BP_Projectiles_Arrow_C" (`KismetMathLibrary.MakeTransform` _returnvalue_location _returnvalue_rotation) "AlwaysSpawn" "MultiplyWithRoot" self null))

(fn `GetHealed`
  (params (IncreaseAmount :type "Float (double-precision)"))
  (`/Game/Dynamic/Blueprints/Components/BPC_Health.IncreaseHealth` (`self.BPC_Health`) IncreaseAmount)
  (`/Game/Dynamic/Widgets/WBP_HealthBox.UpdateCurrentHealth` (`/Game/Dynamic/Widgets/WBP_MainHUD.WBP_HealthBox` (`self.MainHUD`)) (`/Game/Dynamic/Blueprints/Components/BPC_Health.CurrentHealth` (`self.BPC_Health`))))

(fn `UserConstructionScript`
  (`parent.UserConstructionScript`))