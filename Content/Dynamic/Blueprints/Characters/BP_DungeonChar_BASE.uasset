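; BP_DungeonChar_BASE is a base dungeon character with sprite visuals that handles taking damage and hit feedback.
; Damage that BPCHealth allows reduces health, plays a sound, triggers timeline-driven knockback and a red flash, then calls HandleHitExtended, an empty extension hook.
; A character attacker gets hit stop by briefly zeroing its CustomTimeDilation.
; Invincibility expiry stops sprite flicker and restores the hurtbox; CanAct gates actions on defeat, stun and attack state.
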(event `self.ReceiveBeginPlay`
  (add `/Game/Dynamic/Blueprints/Components/BPC_Health.InvincibilityExpired` (`self.BPC_Health`) (delegate `OnInvincibilityExpired`)))

(event `OnInvincibilityExpired`
  (`KismetSystemLibrary.K2_ClearAndInvalidateTimerHandle` (`self.FlickerHandler`))
  (`SceneComponent.SetVisibility` (`self.Sprite`) true false)
  (`PrimitiveComponent.SetCollisionEnabled` (`self.Hurtbox`) "QueryOnly"))

(event `self.ReceiveAnyDamage`
  (params (Damage :type "Float (single-precision)") (DamageType :type "DamageType Object Reference") (InstigatedBy :type "Controller Object Reference") (DamageCauser :type "Actor Object Reference"))
  (if (`/Game/Dynamic/Blueprints/Components/BPC_Health.CanBeDamaged` (`self.BPC_Health`))
    (`/Game/Dynamic/Blueprints/Components/BPC_Health.DecreaseHealth` (`self.BPC_Health`) Damage)
    (`GameplayStatics.PlaySound2D` (`self.HitSound`) 1.0 1.0 0.0 null null)
    (`self.GetKnockedBack` DamageCauser)
    (`self.FlashSprite`)
    (`self.HandleHitExtended`)
    (bind _asbp_dungeon_char_base (cast `/Game/Dynamic/Blueprints/Characters/BP_DungeonChar_BASE` DamageCauser))
    (`self.HitStop` _asbp_dungeon_char_base)))

(event `GetKnockedBack`
  (params (Attacker :type "Actor Object Reference"))
  (bind _output_get (set `self.KnockbackDirection` (`KismetMathLibrary.GetForwardVector` (`KismetMathLibrary.FindLookAtRotation` (`self.K2_GetActorLocation` Attacker) (`self.K2_GetActorLocation`)))))
  (`TimelineComponent.SetPlayRate` (`self.KnockBackMovement`) 5.0)
  (`Timeline|KnockBackMovement` :!via `PlayFromStart`
    (:`Update`
      (set `MovementComponent.Velocity` (* _output_get (`self.KnockbackStrength`) (`GameplayStatics.GetWorldDeltaSeconds`)) (`self.CharacterMovement`)))))

(event `FlashSprite`
  (`PaperFlipbookComponent.SetSpriteColor` (`self.Sprite`) (struct :`R` 1.0 :`A` 1.0))
  (`KismetSystemLibrary.RetriggerableDelay` (`self.FlashDuration`))
  (`PaperFlipbookComponent.SetSpriteColor` (`self.Sprite`) (struct :`R` 1.0 :`G` 1.0 :`B` 1.0 :`A` 1.0)))

(event `HitStop`
  (set `self.CustomTimeDilation` 0.0)
  (`KismetSystemLibrary.RetriggerableDelay` (`self.HitStopDuration`))
  (set `self.CustomTimeDilation` 1.0))

(fn `Can Act`
  (returns (ReturnValue :type Boolean))
  (return (and (not (`/Game/Dynamic/Blueprints/Components/BPC_Health.IsDefeated` (`self.BPC_Health`))) (not (`self.isStunned`)) (not (`self.isAttacking`)))))

(fn `HandleHitExtended`)

(fn `SetSpriteVisibility`
  (`SceneComponent.SetVisibility` (`self.Sprite`) (not (`SceneComponent.bVisible` (`self.Sprite`))) false))

(fn `UserConstructionScript`)